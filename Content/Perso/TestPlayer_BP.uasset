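; TestPlayer_BP is a test player character with camera-relative movement, look controls and a slide-like crouch.
; Axis inputs drive movement along the camera's forward and right vectors and rotate the controller's pitch and yaw.
; Holding C crouches, halves the capsule height and sets crouched max speed to the current speed.
; Tick forces forward input while crouched and prints velocity magnitude for debugging.
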(event `InputAxis|MoveForward`
  (params (AxisValue :type "Float (single-precision)"))
  (`self.AddMovementInput` (`SceneComponent.GetForwardVector` (`self.Camera`)) AxisValue))

(event `InputAxis|MoveRight`
  (params (AxisValue :type "Float (single-precision)"))
  (`self.AddMovementInput` (`SceneComponent.GetRightVector` (`self.Camera`)) AxisValue))

(event `InputAxis|LookUp`
  (params (AxisValue :type "Float (single-precision)"))
  (`self.AddControllerPitchInput` AxisValue))

(event `InputAxis|Turn`
  (params (AxisValue :type "Float (single-precision)"))
  (`self.AddControllerYawInput` AxisValue))

(event `Key|C`
  (params (Key :type "Key Structure"))
  (:`Pressed`
    (set `CharacterMovementComponent.MaxWalkSpeedCrouched` (`KismetMathLibrary.VSize` (`self.GetVelocity`)) (`self.CharacterMovement`))
    (`CapsuleComponent.SetCapsuleHalfHeight` (`self.CapsuleComponent`) 44.0 true)
    (`self.Crouch`)
    (set `self.IsCrouched` true))
  (:`Released`
    (`CapsuleComponent.SetCapsuleHalfHeight` (`self.CapsuleComponent`) 88.0 true)
    (`self.UnCrouch`)
    (set `self.IsCrouched` false)))

(event `self.ReceiveTick`
  (params (DeltaSeconds :type "Float (single-precision)"))
  (`|ExecutionSequence`
    (:`then_0`
      (if (`self.IsCrouched`)
        (`self.AddMovementInput` (`SceneComponent.GetForwardVector` (`self.Camera`)))))
    (:`then_1`
      (`KismetSystemLibrary.PrintString` (`KismetStringLibrary.Conv_DoubleToString` (`KismetMathLibrary.VSize` (`self.GetVelocity`))) true true (struct :`G` 0.66 :`B` 1.0 :`A` 1.0) 0.1))))

(fn `UserConstructionScript`)